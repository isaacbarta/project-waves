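; BP_WavesCompleteController is a controller for the game-complete screen in ProjectWaves.
; On BeginPlay it sets the view to the first CameraActor found in the level and adds the WBP_GameComplete widget to the viewport.
; It also defines helpers to register the default Enhanced Input mapping and to trace under the cursor for BPI_Interactable actors, but neither is called in this Blueprint.
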(event `self.ReceiveBeginPlay`
  (bind _outactors (`GameplayStatics.GetAllActorsOfClass` "/Script/Engine.CameraActor"))
  (`self.SetViewTargetWithBlend` (`|GetArrayItem` _outactors))
  (bind _returnvalue (`|CreateWidget` "/Game/ProjectWaves/UI/MainMenu/WBP_GameComplete.WBP_GameComplete_C" self))
  (`UserWidget.AddToViewport` _returnvalue 0))

(fn `GetClickedItem`
  (returns (bSuccess :type Boolean) (HitActor :type "Actor Object Reference"))
  (bind (_hitresult _returnvalue) (`self.GetHitResultUnderCursorByChannel` "TraceTypeQuery3"))
  (bind (_bblockinghit _binitialoverlap _time _distance _location _impactpoint _normal _impactnormal _physmat _hitactor) (`GameplayStatics.BreakHitResult` _hitresult))
  (return (and _returnvalue (`KismetSystemLibrary.DoesImplementInterface` _hitactor "/Game/ProjectWaves/Blueprints/Interfaces/BPI_Interactable.BPI_Interactable_C")) _hitactor))

(fn `SetupInput`
  (bind _returnvalue (subsystem `EnhancedInputLocalPlayerSubsystem`))
  (`/Engine/EditorBlueprintResources/StandardMacros.IsValid` _returnvalue
    (:`Is Valid`
      (`EnhancedInputSubsystemInterface.AddMappingContext` _returnvalue "/Game/ProjectWaves/Blueprints/Inputs/InputActions/IMC_Default.IMC_Default" 0 (struct)))))

(fn `UserConstructionScript`)