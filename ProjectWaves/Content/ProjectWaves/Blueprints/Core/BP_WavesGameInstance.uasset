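; Game instance that owns the single save slot for level progress and audio settings.
; On init it loads or creates a BP_SaveGame, then signals OnSaveLoaded after a short delay.
; Saving a level stores the next entry in LevelPaths and increments a completed counter, while deleting resets both to the start.
; Audio saves store master, music and SFX values, and every change writes straight to the slot.
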(event `self.ReceiveInit`
  (`self.LoadSaveData`))

(event `/Game/ProjectWaves/Blueprints/Interfaces/BPI_SaveGame.LoadSaveData`
  (bind _returnvalue (`GameplayStatics.DoesSaveGameExist` (`self.SlotName`)))
  (if _returnvalue
    (bind _returnvalue_2 (`GameplayStatics.LoadGameFromSlot` (`self.SlotName`)))
    (bind _asbp_save_game (cast `/Game/ProjectWaves/Blueprints/SaveSystem/BP_SaveGame` _returnvalue_2))
    (set `self.SavedData` _asbp_save_game)
    (`KismetSystemLibrary.Delay` 0.2)
    (`self.OnSaveLoaded`)
    (else
      (bind _returnvalue_3 (`GameplayStatics.CreateSaveGameObject` "/Game/ProjectWaves/Blueprints/SaveSystem/BP_SaveGame.BP_SaveGame_C"))
      (bind _output_get (set `self.SavedData` _returnvalue_3))
      (set `/Game/ProjectWaves/Blueprints/SaveSystem/BP_SaveGame.CurrentLevelName` "None" _output_get)
      (`KismetSystemLibrary.Delay` 0.2)
      (`self.OnSaveLoaded`))))

(event `/Game/ProjectWaves/Blueprints/Interfaces/BPI_SaveGame.SaveGameData`
  (`GameplayStatics.SaveGameToSlot` (`self.SavedData`) (`self.SlotName`)))

(event `/Game/ProjectWaves/Blueprints/Interfaces/BPI_SaveGame.SaveLevel`
  (params (CurrentLevelName :type String) (Async :type Boolean))
  (bind _levelpaths (`self.LevelPaths`))
  (set `/Game/ProjectWaves/Blueprints/SaveSystem/BP_SaveGame.CurrentLevelName` (`|GetArrayItem` _levelpaths (+ (`KismetArrayLibrary.Array_Find` _levelpaths CurrentLevelName) 1)) (`self.SavedData`))
  (set `self.LevelsCompleted` (+ (`self.LevelsCompleted`) 1))
  (`self.SaveGameData`))

(event `/Game/ProjectWaves/Blueprints/Interfaces/BPI_SaveGame.DeleteSave`
  (set `/Game/ProjectWaves/Blueprints/SaveSystem/BP_SaveGame.CurrentLevelName` (`|GetArrayItem` (`self.LevelPaths`)) (`self.SavedData`))
  (set `self.LevelsCompleted` 0)
  (`self.SaveGameData`))

(event `/Game/ProjectWaves/Blueprints/Interfaces/BPI_SaveGame.SaveAudio`
  (params (Master :type "Float (double-precision)") (Music :type "Float (double-precision)") (SFX :type "Float (double-precision)"))
  (bind _saveddata (`self.SavedData`))
  (set `/Game/ProjectWaves/Blueprints/SaveSystem/BP_SaveGame.MasterSound` Master _saveddata)
  (set `/Game/ProjectWaves/Blueprints/SaveSystem/BP_SaveGame.MusicSound` Music _saveddata)
  (set `/Game/ProjectWaves/Blueprints/SaveSystem/BP_SaveGame.SFXSound` SFX _saveddata)
  (`self.SaveGameData`))

(fn `GetSaveData`
  (returns (SavedData :type "/Game/ProjectWaves/Blueprints/SaveSystem/BP_SaveGame Object Reference"))
  (return (`self.SavedData`)))