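; Player controller for the Waves game that handles click-based tile selection and creates the game UI.
; On BeginPlay it adds the input mapping, views through the first CameraActor found, shows the HUD and binds BP_Finish's level-finished event to display the level-complete widget.
; Clicks deselect the current tile, then trace under the cursor for a BPI_Interactable actor to select, with re-clicking the selected tile clearing it.
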(event `self.ReceiveBeginPlay`
  (`self.SetupInput`)
  (bind _outactors (`GameplayStatics.GetAllActorsOfClass` "/Script/Engine.CameraActor"))
  (`self.SetViewTargetWithBlend` (`|GetArrayItem` _outactors))
  (bind _returnvalue (`|CreateWidget` "/Game/ProjectWaves/UI/Game/WBP_GameUI.WBP_GameUI_C" self))
  (`UserWidget.AddToViewport` _returnvalue 0)
  (bind _returnvalue_2 (`GameplayStatics.GetActorOfClass` "/Game/ProjectWaves/Blueprints/Prototyping/BP_Finish.BP_Finish_C"))
  (bind _output_get (set `self.FinishRef` _returnvalue_2))
  (add `/Game/ProjectWaves/Blueprints/Prototyping/BP_Finish.OnLevelFinished` _output_get (delegate `OnLevelFinished_Event`)))

(event `OnLevelFinished_Event`
  (bind _returnvalue (`|CreateWidget` "/Game/ProjectWaves/UI/Game/WBP_LevelComplete.WBP_LevelComplete_C" self))
  (`UserWidget.AddToViewport` _returnvalue 0))

(event `EnhancedInput|/Game/ProjectWaves/Blueprints/Inputs/InputActions/IA_Click`
  (params (ActionValue :type Boolean) (ElapsedSeconds :type "Float (double-precision)") (TriggeredSeconds :type "Float (double-precision)") (InputAction :type "InputAction Object Reference" :default "/Game/ProjectWaves/Blueprints/Inputs/InputActions/IA_Click.IA_Click"))
  (bind (_bsuccess _hitactor) (`self.GetClickedItem`))
  (:`Triggered`
    (`|ExecutionSequence`
      (:`then_0`
        ; If a tile is already selected, deselect it
        (bind _selectedtile (`self.SelectedTile`)
          (:`then`
            (message `/Game/ProjectWaves/Blueprints/Interfaces/BPI_Interactable.OnInteract` _selectedtile false))
          (:`else`)))
      (:`then_1`
        ; Select clicked tile
        (if _bsuccess
          (if (== _hitactor (`self.SelectedTile`))
            (set `self.SelectedTile` null)
            (else
              (bind _output_get (set `self.SelectedTile` _hitactor))
              (message `/Game/ProjectWaves/Blueprints/Interfaces/BPI_Interactable.OnInteract` _output_get true))))))))

(fn `GetClickedItem`
  (returns (bSuccess :type Boolean) (HitActor :type "Actor Object Reference"))
  (bind (_hitresult _returnvalue) (`self.GetHitResultUnderCursorByChannel` "TraceTypeQuery3"))
  (bind (_bblockinghit _binitialoverlap _time _distance _location _impactpoint _normal _impactnormal _physmat _hitactor) (`GameplayStatics.BreakHitResult` _hitresult))
  (return (and _returnvalue (`KismetSystemLibrary.DoesImplementInterface` _hitactor "/Game/ProjectWaves/Blueprints/Interfaces/BPI_Interactable.BPI_Interactable_C")) _hitactor))

(fn `SetupInput`
  (bind _returnvalue (subsystem `EnhancedInputLocalPlayerSubsystem`))
  (`/Engine/EditorBlueprintResources/StandardMacros.IsValid` _returnvalue
    (:`Is Valid`
      (`EnhancedInputSubsystemInterface.AddMappingContext` _returnvalue "/Game/ProjectWaves/Blueprints/Inputs/InputActions/IMC_Default.IMC_Default" 0 (struct)))))

(fn `UserConstructionScript`)