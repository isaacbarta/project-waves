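; Grid tile actor that shows interactable and selection states through emissive color and can hold one spawned object.
; InitializeTile sets the mesh, attaches to the owning actor and offsets itself by row, column and mesh bounds.
; A dynamic material drives the color, which OnInteract changes on interactable tiles.
; RefreshTile rebuilds mesh and material, then spawns the starting object through AttachObject, which replaces any existing one.
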(event `self.ReceiveBeginPlay`
  (`self.CreateMIDynamic`))

(event `self.ReceiveTick`
  (params (DeltaSeconds :type "Float (single-precision)")))

(fn `AttachObject`
  (params (ActorToAttach :type "Actor Class Reference"))
  (`self.DestroyObject`)
  (bind _returnvalue (`|SpawnActorFromClass` ActorToAttach (`KismetMathLibrary.MakeTransform` (+ (`SceneComponent.K2_GetComponentLocation` (`self.TileMesh`)) (`KismetMathLibrary.MakeVector` 0.0 0.0 (`self.ObjectOffset`)))) "Undefined" "MultiplyWithRoot" null null))
  (bind _output_get (set `self.AttachedObject` _returnvalue))
  (`self.K2_AttachToActor` _output_get self "None" "KeepWorld" "SnapToTarget" "KeepRelative" true))

(fn `CreateMIDynamic`
  (bind _returnvalue (`PrimitiveComponent.CreateDynamicMaterialInstance` (`self.TileMesh`) 1 "/Game/ProjectWaves/Assets/Materials/Tiles/MI_EmissiveTile.MI_EmissiveTile" "None"))
  (set `self.MIDynamic` _returnvalue)
  (`self.SetTileColor` (`self.InteractableTileColor`) (`self.NonInteractableTileColor`) (`self.IsInteractableTile`)))

(fn `DestroyObject`
  (returns (DestroyedObject :type "Actor Class Reference"))
  (locals (NewLocalVar :type "Actor Class Reference"))
  (bind _attachedobject (`self.AttachedObject`)
    (:`then`
      (`self.K2_DestroyActor` _attachedobject)
      (set `local.NewLocalVar` (`GameplayStatics.GetObjectClass` _attachedobject))
      (set `self.AttachedObject` null)
      (return (`local.NewLocalVar`)))
    (:`else`)))

(fn `InitializeTile`
  (bind _returnvalue (`self.GetOwner`))
  (`|ExecutionSequence`
    (:`then_0`
      ; Set static mesh and create Dynamic MI
      (`StaticMeshComponent.SetStaticMesh` (`self.TileMesh`) (`self.Mesh`))
      (`self.CreateMIDynamic`))
    (:`then_1`
      ; If Generator is valid, attach tile to it
      (`/Engine/EditorBlueprintResources/StandardMacros.IsValid` _returnvalue
        (:`Is Valid`
          (`self.K2_AttachToActor` _returnvalue "None" "SnapToTarget" "SnapToTarget" "KeepRelative" false))))
    (:`then_2`
      ; Set location of tile
      (`self.K2_SetActorRelativeLocation` (`KismetMathLibrary.MakeVector` (* (.x (`.BoxExtent` (`KismetSystemLibrary.GetComponentBounds` (`self.TileMesh`)))) (`self.Column`) 2.0) (* (.y (`.BoxExtent` (`KismetSystemLibrary.GetComponentBounds` (`self.TileMesh`)))) (`self.Row`) 2.0))))))

(fn `OnInteract`
  (params (bIsSelected :type Boolean))
  (returns (bSuccess :type Boolean))
  (if (`self.IsInteractableTile`)
    (`self.SetTileColor` (`self.SelectedTileColor`) (`self.InteractableTileColor`) (`local.bIsSelected`))
    (set `self.IsTileSelected` (`local.bIsSelected`))
    (return true)))

(fn `RefreshTile`
  (`|ExecutionSequence`
    (:`then_0`
      ; Set new static mesh
      (`StaticMeshComponent.SetStaticMesh` (`self.TileMesh`) (`self.Mesh`)))
    (:`then_1`
      ; Create new MI
      (`self.CreateMIDynamic`))
    (:`then_2`
      ; Attach starting object
      (`self.AttachObject` (`self.StartingObject`)))))

(fn `SetTileColor`
  (params (ColorA :type "LinearColor Structure") (ColorB :type "LinearColor Structure") (ShouldPickA :type Boolean))
  (bind _midynamic (`self.MIDynamic`)
    (:`then`
      (`MaterialInstanceDynamic.SetVectorParameterValue` _midynamic "Emissive Color" (`KismetMathLibrary.SelectColor` ColorA ColorB ShouldPickA)))
    (:`else`)))

(fn `UserConstructionScript`)