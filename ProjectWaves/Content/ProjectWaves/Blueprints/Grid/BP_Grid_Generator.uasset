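; BP_Grid_Generator spawns a rows-by-columns grid of BP_Grid_Tile actors and manages placing objects on them from a limited stock.
; InitializeTiles clears existing tiles, then spawns and initializes new ones with their row, column and mesh.
; Place and remove functions scan attached tiles for selected ones, attach or destroy objects, and update remaining counts in the AvailableObjects map.
; Removal also broadcasts OnObjectRemoved with the new count.
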(fn `ClearTiles`
  (bind _currenttiles (`self.CurrentTiles`))
  (if (> (`KismetArrayLibrary.Array_Length` (`self.CurrentTiles`)) 0)
    (bind (_arrayindex _arrayelement) (`/Engine/EditorBlueprintResources/StandardMacros.ReverseForEachLoop` _currenttiles)
      (:`LoopBody`
        (`self.K2_DestroyActor` _arrayelement))
      (:`Completed`
        (`KismetArrayLibrary.Array_Clear` _currenttiles)))))

(fn `InitializeTiles`
  (`self.ClearTiles`)
  (for _index (range (`self.Rows`))
    (for _index_2 (range (`self.Columns`))
      (bind _returnvalue (`|SpawnActorFromClass` "/Game/ProjectWaves/Blueprints/Grid/BP_Grid_Tile.BP_Grid_Tile_C" (`KismetMathLibrary.MakeTransform` (`self.K2_GetActorLocation`) (`self.K2_GetActorRotation`)) "AlwaysSpawn" "MultiplyWithRoot" self _index _index_2 (`self.TileMesh`) null))
      (`/Game/ProjectWaves/Blueprints/Grid/BP_Grid_Tile.InitializeTile` _returnvalue)
      (`KismetArrayLibrary.Array_Add` (`self.CurrentTiles`) _returnvalue))))

(fn `PlaceObjectOnTile`
  (params (ActorRef :type "Actor Class Reference"))
  (returns (NewAmount :type Integer) (WasObjectAttached :type Boolean))
  (locals (ObjectAttached :type Boolean) (ObjectValue :type Integer))
  (bind _actorref (`local.ActorRef`))
  (bind _returnvalue (- (`local.ObjectValue`) 1))
  ; Get attached tiles and loop through them
  (for _array_element (`self.GetAttachedActors` self true false)
    ; Check if tile is selected
    (bind _asbp_grid_tile (cast `/Game/ProjectWaves/Blueprints/Grid/BP_Grid_Tile` _array_element))
    (if (`/Game/ProjectWaves/Blueprints/Grid/BP_Grid_Tile.IsTileSelected` _asbp_grid_tile)
      ; Find object in available objects and attach it
      (bind _output_get (set `local.ObjectValue` (`BlueprintMapLibrary.Map_Find` (`self.AvailableObjects`) _actorref)))
      (if (> _output_get 0)
        (`/Game/ProjectWaves/Blueprints/Grid/BP_Grid_Tile.AttachObject` _asbp_grid_tile _actorref)
        (set `local.ObjectAttached` true))))
  ; If object was attached
  (if (`local.ObjectAttached`)
    ;; Set new value for object
    (`BlueprintMapLibrary.Map_Add` (`self.AvailableObjects`) (`local.ActorRef`) _returnvalue)
    (return _returnvalue (`local.ObjectAttached`))))

(fn `RemoveObjectFromTile`
  (returns (NewAmount :type Integer) (RemovedObject :type "Actor Class Reference"))
  (locals (ObjectAttached :type Boolean :default true) (ObjectValue :type Integer) (DestroyedObject :type "Actor Class Reference"))
  (bind _destroyedobject (`local.DestroyedObject`))
  (bind _availableobjects (`self.AvailableObjects`))
  ; Get attached tiles and loop through them
  (for _array_element (`self.GetAttachedActors` self true false)
    ; Check if tile is selected
    (bind _asbp_grid_tile (cast `/Game/ProjectWaves/Blueprints/Grid/BP_Grid_Tile` _array_element))
    (if (`/Game/ProjectWaves/Blueprints/Grid/BP_Grid_Tile.IsTileSelected` _asbp_grid_tile)
      ; Find object in available objects and destroy it
      (bind _destroyedobject_2 (`/Game/ProjectWaves/Blueprints/Grid/BP_Grid_Tile.DestroyObject` _asbp_grid_tile))
      (set `local.ObjectAttached` false)
      (set `local.DestroyedObject` _destroyedobject_2)))
  ; If object was removed
  (if (not (`local.ObjectAttached`))
    ;; Set new value for object
    (bind _output_get (set `local.ObjectValue` (`BlueprintMapLibrary.Map_Find` _availableobjects _destroyedobject)))
    (bind _returnvalue (+ _output_get 1))
    (`BlueprintMapLibrary.Map_Add` _availableobjects _destroyedobject _returnvalue)
    (`self.OnObjectRemoved` _returnvalue (`local.DestroyedObject`))
    (return _returnvalue (`local.DestroyedObject`))))

(fn `UserConstructionScript`)