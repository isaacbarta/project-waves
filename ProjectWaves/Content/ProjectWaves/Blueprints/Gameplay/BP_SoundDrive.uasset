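; BP_SoundDrive is a gameplay actor with a progress display and six edge and corner kill boxes that absorb soundwaves.
; On BeginPlay it copies its Progress and SequenceText values once into the WBP_DriveProgress hosted by its Widget component.
; Each kill box destroys any overlapping BP_Soundwave, using the same soft-class check repeated per box.
; The overlaps only destroy the wave and do not change the drive's progress.
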(event `self.ReceiveBeginPlay`
  (bind _aswbp_drive_progress (cast `/Game/ProjectWaves/UI/Game/WBP_DriveProgress` (`WidgetComponent.GetWidget` (`self.Widget`))))
  (set `/Game/ProjectWaves/UI/Game/WBP_DriveProgress.Progress` (`self.Progress`) _aswbp_drive_progress)
  (set `/Game/ProjectWaves/UI/Game/WBP_DriveProgress.SeqText` (`self.Sequence Text`) _aswbp_drive_progress))

(event `self.TopKillBox.OnComponentBeginOverlap`
  (params (OverlappedComponent :type "PrimitiveComponent Object Reference") (OtherActor :type "Actor Object Reference") (OtherComp :type "PrimitiveComponent Object Reference") (OtherBodyIndex :type Integer) (bFromSweep :type Boolean) (SweepResult :type "HitResult Structure (by ref)"))
  (`KismetSystemLibrary.IsObjectOfSoftClass` OtherActor "/Game/ProjectWaves/Blueprints/Gameplay/BP_Soundwave.BP_Soundwave_C"
    (:`True`
      (`self.K2_DestroyActor` OtherActor))))

(event `self.TopRightKillBox.OnComponentBeginOverlap`
  (params (OverlappedComponent :type "PrimitiveComponent Object Reference") (OtherActor :type "Actor Object Reference") (OtherComp :type "PrimitiveComponent Object Reference") (OtherBodyIndex :type Integer) (bFromSweep :type Boolean) (SweepResult :type "HitResult Structure (by ref)"))
  (`KismetSystemLibrary.IsObjectOfSoftClass` OtherActor "/Game/ProjectWaves/Blueprints/Gameplay/BP_Soundwave.BP_Soundwave_C"
    (:`True`
      (`self.K2_DestroyActor` OtherActor))))

(event `self.RightKillBox.OnComponentBeginOverlap`
  (params (OverlappedComponent :type "PrimitiveComponent Object Reference") (OtherActor :type "Actor Object Reference") (OtherComp :type "PrimitiveComponent Object Reference") (OtherBodyIndex :type Integer) (bFromSweep :type Boolean) (SweepResult :type "HitResult Structure (by ref)"))
  (`KismetSystemLibrary.IsObjectOfSoftClass` OtherActor "/Game/ProjectWaves/Blueprints/Gameplay/BP_Soundwave.BP_Soundwave_C"
    (:`True`
      (`self.K2_DestroyActor` OtherActor))))

(event `self.BottomKillBox.OnComponentBeginOverlap`
  (params (OverlappedComponent :type "PrimitiveComponent Object Reference") (OtherActor :type "Actor Object Reference") (OtherComp :type "PrimitiveComponent Object Reference") (OtherBodyIndex :type Integer) (bFromSweep :type Boolean) (SweepResult :type "HitResult Structure (by ref)"))
  (`KismetSystemLibrary.IsObjectOfSoftClass` OtherActor "/Game/ProjectWaves/Blueprints/Gameplay/BP_Soundwave.BP_Soundwave_C"
    (:`True`
      (`self.K2_DestroyActor` OtherActor))))

(event `self.BottomLeftKillBox.OnComponentBeginOverlap`
  (params (OverlappedComponent :type "PrimitiveComponent Object Reference") (OtherActor :type "Actor Object Reference") (OtherComp :type "PrimitiveComponent Object Reference") (OtherBodyIndex :type Integer) (bFromSweep :type Boolean) (SweepResult :type "HitResult Structure (by ref)"))
  (`KismetSystemLibrary.IsObjectOfSoftClass` OtherActor "/Game/ProjectWaves/Blueprints/Gameplay/BP_Soundwave.BP_Soundwave_C"
    (:`True`
      (`self.K2_DestroyActor` OtherActor))))

(event `self.LeftKillBox.OnComponentBeginOverlap`
  (params (OverlappedComponent :type "PrimitiveComponent Object Reference") (OtherActor :type "Actor Object Reference") (OtherComp :type "PrimitiveComponent Object Reference") (OtherBodyIndex :type Integer) (bFromSweep :type Boolean) (SweepResult :type "HitResult Structure (by ref)"))
  (`KismetSystemLibrary.IsObjectOfSoftClass` OtherActor "/Game/ProjectWaves/Blueprints/Gameplay/BP_Soundwave.BP_Soundwave_C"
    (:`True`
      (`self.K2_DestroyActor` OtherActor))))

(fn `UserConstructionScript`)