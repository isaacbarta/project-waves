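; BP_Finish is the level's finish object, which signals completion and shows its state through a glowing material.
; BeginPlay creates a dynamic glow material on the static mesh, which Finish turns green and Break turns red.
; Finish is guarded to complete only once: it calls the empty TimeDelay event, fires OnLevelFinished and saves the current level through the GameInstance.
; Overlap and Tick are unused, so Finish and Break must be triggered externally.
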(event `self.ReceiveBeginPlay`
  (set `self.HasFinished` false)
  (bind _returnvalue (`PrimitiveComponent.CreateDynamicMaterialInstance` (`self.StaticMesh`) 1 "/Game/ProjectWaves/Assets/Materials/StartFinish/MI_Finish_Glow.MI_Finish_Glow" "None"))
  (set `self.DynamicMI` _returnvalue))

(event `Finish`
  (if (not (`self.HasFinished`))
    (`MaterialInstanceDynamic.SetVectorParameterValue` (`self.DynamicMI`) "Emissive Color" (struct :`G` 1.0 :`A` 1.0))
    (`self.TimeDelay`)
    (`self.OnLevelFinished`)
    (set `self.HasFinished` true)
    (bind _returnvalue (`GameplayStatics.GetCurrentLevelName` true))
    (message `/Game/ProjectWaves/Blueprints/Interfaces/BPI_SaveGame.SaveLevel` (`GameplayStatics.GetGameInstance`) _returnvalue false)))

(event `Break`
  (`MaterialInstanceDynamic.SetVectorParameterValue` (`self.DynamicMI`) "Emissive Color" (struct :`R` 1.0 :`A` 1.0)))

(event `TimeDelay`)

(fn `UserConstructionScript`)