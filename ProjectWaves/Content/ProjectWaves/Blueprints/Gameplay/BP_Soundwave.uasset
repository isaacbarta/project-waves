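; BP_Soundwave is a soundwave actor that triggers the finish object when it overlaps it.
; On overlap, it checks the other actor for BPI_Finish, casts it to BP_Finish, calls Finish, then destroys itself after a short delay.
; An OnDestroyed handler, bound at BeginPlay, also destroys its Niagara component.
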(event `self.ReceiveBeginPlay`
  (add `self.OnDestroyed` (delegate `OnDestroyed_Event`)))

(event `OnDestroyed_Event` :!signature `self.OnDestroyed`
  (params (DestroyedActor :type "Actor Object Reference"))
  (`ActorComponent.K2_DestroyComponent` (`self.Niagara`)))

(event `self.ReceiveActorBeginOverlap`
  (params (OtherActor :type "Actor Object Reference"))
  (if (`KismetSystemLibrary.DoesImplementInterface` OtherActor "/Game/ProjectWaves/Blueprints/Prototyping/BPI_Finish.BPI_Finish_C")
    (bind _asbp_finish (cast `/Game/ProjectWaves/Blueprints/Gameplay/BP_Finish` OtherActor))
    (`/Game/ProjectWaves/Blueprints/Gameplay/BP_Finish.Finish` _asbp_finish)
    (`KismetSystemLibrary.Delay` 0.2)
    (`self.K2_DestroyActor`)))

(fn `UserConstructionScript`)