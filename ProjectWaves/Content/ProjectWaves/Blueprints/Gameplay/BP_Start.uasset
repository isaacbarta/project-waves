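; BP_Start is a sound emitter that repeatedly spawns BP_Soundwave actors at its SoundStart component's transform.
; Tick feeds a one-second Delay, so a wave spawns roughly every second rather than every frame.
; An unconnected line-trace chain, which never runs, would trace forward from SoundStart and call Mirror on a hit BP_Reflector or Finish on a BP_Finish, selected by interface checks.
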(event `self.ReceiveTick`
  (params (DeltaSeconds :type "Float (single-precision)"))
  (`KismetSystemLibrary.Delay` 1.0)
  (`|SpawnActorFromClass` "/Game/ProjectWaves/Blueprints/Gameplay/BP_Soundwave.BP_Soundwave_C" (`SceneComponent.K2_GetComponentToWorld` (`self.SoundStart`)) "Undefined" "MultiplyWithRoot" null null))

(fn `UserConstructionScript`)